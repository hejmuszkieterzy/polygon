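; BP_Plank is a plank the goblin player can pick up by overlapping its box while pressing E.
; Tick re-casts the player character to GoblinBP every frame for the overlap check.
; Pickup snaps it to the RightHandSocket, disables mesh collision, lowers jump velocity and sets IsHoldingChest to false.
; A drop sequence that detaches, spawns a new plank and restores jump and physics is unconnected and never runs.
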(event OnComponentBeginOverlap(Box)
  (params (OverlappedComponent :type Primitive%20Component%20Object%20Reference) (OtherActor :type Actor%20Object%20Reference) (OtherComp :type Primitive%20Component%20Object%20Reference) (OtherBodyIndex :type Integer) (bFromSweep :type Boolean) (SweepResult :type Hit%20Result%20Structure%20%28by%20ref%29))
  (bind _returnvalue (Game|GetPlayerCharacter 0))
  (if (and (Variables|/Game/Goblin/GoblinBP.GoblinBP_C|GetIsPressingE (stale EventTick _asgoblin_bp)) (== OtherActor _returnvalue))
    (Transformation|AttachComponentToComponent (Variables|/Script/Engine.Character|GetMesh _returnvalue) "RightHandSocket" "SnapToTarget" "SnapToTarget" "KeepRelative" true)
    (Collision|SetCollisionEnabled (Variables|Default|GetPlankMesh) "NoCollision")
    (Variables|/Game/Goblin/GoblinBP.GoblinBP_C|SetIs_Holding_Chest (stale EventTick _asgoblin_bp) false)
    (Variables|/Script/Engine.CharacterMovementComponent|SetJumpZVelocity (Variables|/Script/Engine.Character|GetCharacterMovement (stale EventTick _asgoblin_bp)) 2e+02)))

(event EventBeginPlay)

(event EventTick
  (params (DeltaSeconds :type Float%20%28single-precision%29))
  (bind _asgoblin_bp (Utilities|Casting|CastToGoblinBP (Game|GetPlayerCharacter 0))))

(event Collision|EventActorBeginOverlap
  (params (OtherActor :type Actor%20Object%20Reference)))

(fn ConstructionScript)